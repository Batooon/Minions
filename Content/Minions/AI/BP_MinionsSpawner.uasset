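; BP_MinionsSpawner is an actor that spawns a batch of Minion_Character minions at its own location.
; A looping half-second timer starts on BeginPlay and spawns one minion per tick, then invalidates itself once SpawnedAmount reaches MinionsAmount.
; Each minion receives the spawner's team, team color and patrolling line, and always spawns, with its position adjusted if possible to avoid collisions.
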(event Custom|CustomEvent
  (if (>= (Variables|Default|GetSpawnedAmount) (Variables|Default|GetMinionsAmount))
    (Utilities|Time|InvalidateTimerHandle (Variables|Default|GetMinionsSpawn))
    (else
      (CallFunction|SpawnMinion)
      (Math|Integer|IncrementInt (Variables|Default|GetSpawnedAmount)))))

(event EventBeginPlay
  (bind _returnvalue (Utilities|Time|SetTimerbyEvent (delegate Custom|CustomEvent) 0.5 true))
  (Variables|Default|SetMinionsSpawn _returnvalue))

(fn ConstructionScript)

(fn SpawnMinion
  (Game|SpawnActorfromClass "/Game/Minions/AI/Minion_Character.Minion_Character_C" (Transformation|GetActorTransform) "AdjustIfPossibleButAlwaysSpawn" "MultiplyWithRoot" 0 (Utilities|String|StringToName (Variables|Default|GetTeam)) (Variables|Default|GetTeamColor) (Variables|Default|GetLine) 0))