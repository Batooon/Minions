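; BP_LinePath defines an ordered path of point actors, filed under minion AI.
; On BeginPlay it caches the world location of every PathPoints entry into a Locations array.
; GetNextPoint returns the actor after the given point, looping from the last back to the first, and returns the first when the given point is invalid.
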(event EventBeginPlay
  (for _array_element (Variables|Default|GetPathPoints)
    (Utilities|Array|Add (Variables|Default|GetLocations) (Transformation|GetActorLocation _array_element))))

(fn ConstructionScript)

(fn GetNextPoint
  (params (CurrentPoint :type BP%20Line%20Point%20Object%20Reference))
  (bind _pathpoints (Variables|Default|GetPathPoints))
  (bind _returnvalue (Utilities|Array|FindItem _pathpoints CurrentPoint))
  (Utilities|IsValid CurrentPoint
    (:Is%20Valid
      (if (== _returnvalue (Utilities|Array|LastIndex _pathpoints))
        _
        (else
          (return (Utilities|Array|Get(acopy) _pathpoints (+ _returnvalue 1))))))
    (:Is%20Not%20Valid
      _))
  (return (Utilities|Array|Get(acopy) _pathpoints)))